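; BP_Camera is a placeable camera that becomes the player's view when BP_hero enters its trigger box.
; On overlap it registers itself as the hero's NewCamera and switches the view target to itself.
; BeginPlay waits a tick, then applies the same switch if the hero already overlaps the box.
; The construction script positions and sizes the trigger from TriggerTransform and TriggerExtend.
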(event `self.ReceiveBeginPlay`
  (`KismetSystemLibrary.Delay` 0.0)
  (bind _asbp_hero (cast `/Game/Bluebrints/Character/BP_hero` (`GameplayStatics.GetPlayerPawn` 0)))
  (for _array_element (`self.GetOverlappingComponents` _asbp_hero)
    (if (== _array_element (`self.TriggerBox`))
      (set `/Game/Bluebrints/Character/BP_hero.NewCamera` self _asbp_hero)
      (`PlayerController.SetViewTargetWithBlend` (`GameplayStatics.GetPlayerController` 0) self 0.0 "VTBlend_Linear" 0.0 false))))

(event `self.TriggerBox.OnComponentBeginOverlap`
  (params (OverlappedComponent :type "PrimitiveComponent Object Reference") (OtherActor :type "Actor Object Reference") (OtherComp :type "PrimitiveComponent Object Reference") (OtherBodyIndex :type Integer) (bFromSweep :type Boolean) (SweepResult :type "HitResult Structure (by ref)"))
  (bind _asbp_hero (cast `/Game/Bluebrints/Character/BP_hero` OtherActor))
  (set `/Game/Bluebrints/Character/BP_hero.NewCamera` self _asbp_hero)
  (`PlayerController.SetViewTargetWithBlend` (`GameplayStatics.GetPlayerController` 0) self 0.0 "VTBlend_Linear" 0.0 false))

(fn `UserConstructionScript`
  (`SceneComponent.K2_SetRelativeTransform` (`self.TriggerBox`) (`self.TriggerTransform`) false false)
  (`BoxComponent.SetBoxExtent` (`self.TriggerBox`) (`self.TriggerExtend`) true))